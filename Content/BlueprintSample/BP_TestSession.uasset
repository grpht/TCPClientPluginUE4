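; BP_TestSession is a sample network session Blueprint that receives room-entry and chat message responses.
; On start it registers both response packet classes with the session.
; Received packets are switched on packet ID, cast to their response type and rebroadcast through matching event dispatchers.
; Connect and disconnect events print debug strings with hard-wired success branches, while the send and destroy hooks are empty.
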(event `self.OnStartBP`
  ;[1 1 1] Register RecvPacket on start
  (`self.RegisterRecvPacket` "/TCPClientPlugin/BlueprintSample/Packet/BP_TestEnterRoomResponse.BP_TestEnterRoomResponse_C")
  (`self.RegisterRecvPacket` "/TCPClientPlugin/BlueprintSample/Packet/BP_TestChattingMessageResponse.BP_TestChattingMessageResponse_C"))

(event `self.OnSendBP`
  (params (id :type Integer) (contentsByteSize :type Integer))
  ;[1 1 1] For debugging Sending Packet
)

(event `self.OnRecvBP`
  (params (packet :type "TCPRecvPacketBase Object Reference"))
  ;[1 1 1] Process RecvPacket
  (switch `int` (`TCPRecvPacketBase.GetPacketId` packet)
    (:`1`
      (bind _asbp_test_enter_room_response (cast `/TCPClientPlugin/BlueprintSample/Packet/BP_TestEnterRoomResponse` packet))
      (`self.OnEnterRoomResponse` _asbp_test_enter_room_response))
    (:`3`
      (bind _asbp_test_chatting_message_response (cast `/TCPClientPlugin/BlueprintSample/Packet/BP_TestChattingMessageResponse` packet))
      (`self.OnChattingMessageResponse` _asbp_test_chatting_message_response))))

(event `self.OnDestroyBP`)

(event `self.OnConnectedBP`
  (params (success :type Boolean))
  (if true
    (`KismetSystemLibrary.PrintString` null "Connect Success")
    (else
      (`KismetSystemLibrary.PrintString` null "Connect Failed"))))

(event `self.OnDisconnectedBP`
  (params (normalShutdown :type Boolean))
  (if true
    (`KismetSystemLibrary.PrintString` null "Disconnected Nor,a;;u")
    (else
      (`KismetSystemLibrary.PrintString` null "Disconnected With Error"))))