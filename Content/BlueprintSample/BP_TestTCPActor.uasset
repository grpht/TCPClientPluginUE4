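; Sample actor that demonstrates how Blueprints use the TCP client subsystem to manage a session and send packets.
; On BeginPlay it connects a BP_TestSession, caches it on success, and unbinds its connect and disconnect delegates as they fire.
; Unwired example chains show lazy session lookup by name and sending enter-room and chat request packets built with CreateSendPacketBP.
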(event `OnConnected`
  (params (SessionName :type String) (Success :type Boolean) (ReturnSession :type "TCPSessionBase Object Reference"))
  ;[1 1 1] ConnectSession
  (bind _asbp_test_session (cast `/TCPClientPlugin/BlueprintSample/BP_TestSession` ReturnSession))
  (remove `TCPClientSubsystem.OnConnected` (subsystem `TCPClientSubsystem`) (delegate `OnConnected`))
  (if Success
    (set `self.Session` _asbp_test_session)))

(event `self.ReceiveBeginPlay`
  ;[1 1 1] ConnectSession
  (`TCPClientSubsystem.ConnectSession` (subsystem `TCPClientSubsystem`) "/TCPClientPlugin/BlueprintSample/BP_TestSession.BP_TestSession_C" (delegate `OnConnected`) (delegate `OnDisconnected`)))

(event `OnDisconnected`
  (params (SessionName :type String) (NormalShutdown :type Boolean))
  ;[1 1 1] ConnectSession
  (if (`KismetStringLibrary.EqualEqual_StrStr` SessionName "Test")
    (remove `TCPClientSubsystem.OnDisconnected` (subsystem `TCPClientSubsystem`) (delegate `OnDisconnected`))))

(event `OnGetLazy`
  (params (SessionName :type String) (Success :type Boolean) (ReturnSession :type "TCPSessionBase Object Reference"))
  ;[1 1 1] Get session, When you're not sure if session is connected
  (bind _asbp_test_session (cast `/TCPClientPlugin/BlueprintSample/BP_TestSession` ReturnSession))
  (remove `TCPClientSubsystem.OnConnected` (subsystem `TCPClientSubsystem`) (delegate `OnGetLazy`))
  (set `self.Session` _asbp_test_session))

(fn `UserConstructionScript`)